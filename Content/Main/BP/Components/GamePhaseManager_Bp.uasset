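; Game mode component that runs a turn-based quiz match as a timed phase state machine, from lobby through rounds, bonus questions, duels and tiebreakers to a winner.
; Tick watches each phase's duration, then TransitionCheck picks the next phase from question mode, marking results and landing spot effects.
; Entering a phase triggers game mode logic and pushes screen phase and end time to the game state.
; A debug override jumps to any phase.
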(event `self.ReceiveBeginPlay`
  (bind _asgameplay_game_mode_bp (cast `/Game/Main/BP/GameMode/GameplayGameMode_Bp` (`self.GetOwner`))
    (:`then`
      (set `self.OwningGameMode` _asgameplay_game_mode_bp)
      (bind _asgame_play_game_state_bp (cast `/Game/Main/BP/GameState/GamePlayGameState_Bp` (`GameplayStatics.GetGameState`)))
      (set `self.SCGameState` _asgame_play_game_state_bp))
    (:`CastFailed`
      (`KismetSystemLibrary.PrintString` "GAME PHASE NOT IN GAME MODE" true true (struct :`R` 1.0 :`A` 1.0)))))

(event `self.ReceiveTick`
  (params (DeltaSeconds :type "Float (single-precision)"))
  (if (`self.CheckPhaseTime`)
    (`self.PhaseCheck`)))

(fn `Debug_OverridePhase`
  (params (PhaseToGo :type "/Game/Main/Enums/GamePhase_Enum Enum" :default "NewEnumerator0"))
  (bind _currentphase (`self.CurrentPhase`))
  (set `self.CheckPhaseTime` false)
  (`self.OnExitPhase` (`self.CurrentPhase`))
  (set `self.CurrentPhase` (`local.PhaseToGo`))
  (`self.OnEnterPhase` _currentphase)
  (`self.SetPhaseTime` _currentphase)
  (set `self.CheckPhaseTime` true))

(fn `MoveToNextPhase`
  (locals (NewPhase :type "/Game/Main/Enums/GamePhase_Enum Enum"))
  (bind _currentphase (`self.CurrentPhase`))
  (set `self.CheckPhaseTime` false)
  (`self.OnExitPhase` _currentphase)
  (bind _resultphase (`self.TransitionCheck` _currentphase))
  (bind _output_get (set `local.NewPhase` _resultphase))
  (`self.OnEnterPhase` _output_get)
  (`self.SetPhaseTime` (`local.NewPhase`))
  (bind _output_get_2 (set `self.CurrentPhase` (`local.NewPhase`)))
  (if (`|EnumInequality` _output_get_2 "NewEnumerator14")
    (set `self.CheckPhaseTime` true)))

(fn `OnEnterPhase`
  (params (EnteredPhase :type "/Game/Main/Enums/GamePhase_Enum Enum" :default "NewEnumerator0"))
  (bind _owninggamemode (`self.OwningGameMode`))
  (bind _owninggamemode_2 (`self.OwningGameMode`))
  (bind _owninggamemode_3 (`self.OwningGameMode`))
  (`|ExecutionSequence`
    (:`then_0`
      (switch `/Game/Main/Enums/GamePhase_Enum` (`local.EnteredPhase`)
        (:`NewEnumerator0`
          (set `self.CheckPhaseTime` false))
        (:`NewEnumerator1`
          (`/Game/Main/BP/GameMode/GameplayGameMode_Bp.IncrementRoundCount` (`self.OwningGameMode`)))
        (:`NewEnumerator2`
          (`/Game/Main/BP/GameMode/GameplayGameMode_Bp.Round Category Voting ` _owninggamemode_3)
          (set `/Game/Main/BP/GameMode/GameplayGameMode_Bp.AcceptInput` true _owninggamemode_3))
        (:`NewEnumerator3`
          (`/Game/Main/BP/GameMode/GameplayGameMode_Bp.CalculateSelectedCategory` (`self.OwningGameMode`)))
        (:`NewEnumerator19`
          (`/Game/Main/BP/GameMode/GameplayGameMode_Bp.ResetAnsweringPlayerToInitialPlayer` (`self.OwningGameMode`)))
        (:`NewEnumerator4`
          (`/Game/Main/BP/GameMode/GameplayGameMode_Bp.Check and Set Answering Player` (`self.OwningGameMode`)))
        (:`NewEnumerator6`
          (set `/Game/Main/BP/GameMode/GameplayGameMode_Bp.AcceptInput` true (`self.OwningGameMode`)))
        (:`NewEnumerator7`
          (`/Game/Main/BP/GameMode/GameplayGameMode_Bp.MarkPlayersAnswers` (`self.OwningGameMode`)))
        (:`NewEnumerator8`
          (`/Game/Main/BP/GameMode/GameplayGameMode_Bp.Check Landing Spot Effect ` (`self.OwningGameMode`)))
        (:`NewEnumerator9`
          (set `/Game/Main/BP/GameMode/GameplayGameMode_Bp.AcceptInput` true (`self.OwningGameMode`))
          (`/Game/Main/BP/GameMode/GameplayGameMode_Bp.Prepare Duel For Player` (`self.OwningGameMode`)))
        (:`NewEnumerator10`
          (set `/Game/Main/BP/GameMode/GameplayGameMode_Bp.AcceptInput` true (`self.OwningGameMode`))
          (`/Game/Main/BP/GameMode/GameplayGameMode_Bp.SetNextQuestionMode` _owninggamemode_2 "NewEnumerator2")
          (`/Game/Main/BP/PlayerController/GameplayPlayerController_BP.ShowScreen` (`/Game/Main/BP/GameMode/GameplayGameMode_Bp.CurrentAnsweringPlayer` _owninggamemode_2) "NewEnumerator2"))
        (:`NewEnumerator16`
          (`/Game/Main/BP/GameMode/GameplayGameMode_Bp.SetNextQuestionMode` (`self.OwningGameMode`) "NewEnumerator1")
          (if (`/Game/Main/BP/GameMode/GameplayGameMode_Bp.DuelDecision` _owninggamemode)
            (`/Game/Main/BP/GameMode/GameplayGameMode_Bp.NoDuelablePlayer` _owninggamemode)))
        (:`NewEnumerator12`
          (`/Game/Main/BP/GameMode/GameplayGameMode_Bp.SetNextQuestionMode` (`self.OwningGameMode`) "NewEnumerator4"))
        (:`NewEnumerator13`
          (`/Game/Main/BP/GameMode/GameplayGameMode_Bp.Game End Calculate Final Scores` (`self.OwningGameMode`)))
        (:`NewEnumerator14`
          (set `self.CheckPhaseTime` false))))
    (:`then_1`
      (`/Game/Main/BP/GameState/GamePlayGameState_Bp.Set Screen Phase` (`self.SCGameState`) (`local.EnteredPhase`)))))

(fn `OnExitPhase`
  (params (Phase :type "/Game/Main/Enums/GamePhase_Enum Enum" :default "NewEnumerator0")))

(fn `PhaseCheck`
  (if (<= (- (`self.TimeTillNextPhase`) (`KismetSystemLibrary.GetGameTimeInSeconds`)) 0.0)
    (`self.MoveToNextPhase`)))

(fn `SetPhaseTime`
  (params (Phase :type "/Game/Main/Enums/GamePhase_Enum Enum" :default "NewEnumerator0"))
  (bind _output_get (set `self.TimeTillNextPhase` (+ (`BlueprintMapLibrary.Map_Find` (`self.ScreenAndDuration`) (`local.Phase`)) (`KismetSystemLibrary.GetGameTimeInSeconds`))))
  (`/Game/Main/BP/GameState/GamePlayGameState_Bp.Set Phase Time` (`self.SCGameState`) _output_get))

(fn `TransitionCheck`
  (params (PhaseToCheck :type "/Game/Main/Enums/GamePhase_Enum Enum" :default "NewEnumerator0"))
  (returns (ResultPhase :type "/Game/Main/Enums/GamePhase_Enum Enum"))
  (bind _owninggamemode (`self.OwningGameMode`))
  (bind _marksuccessful (`/Game/Main/BP/GameMode/GameplayGameMode_Bp.MarkSuccessful` (`self.OwningGameMode`)))
  (switch `/Game/Main/Enums/GamePhase_Enum` (`local.PhaseToCheck`)
    (:`NewEnumerator0`
      (return "NewEnumerator1"))
    (:`NewEnumerator1`
      (return "NewEnumerator2"))
    (:`NewEnumerator2`
      (set `/Game/Main/BP/GameMode/GameplayGameMode_Bp.AcceptInput` false (`self.OwningGameMode`))
      (return "NewEnumerator3"))
    (:`NewEnumerator3`
      (return "NewEnumerator19"))
    (:`NewEnumerator19`
      (return "NewEnumerator4"))
    (:`NewEnumerator4`
      ;[1 1 1] If question mode is normal check if the current player can answer question if it can process the question and move to next phase else remove status and move to next phase, every other question mode moves processes the question and moves to the next phase
      (switch `/Game/Main/Enums/Question/QuestionMode_Enum` (`/Game/Main/BP/GameMode/GameplayGameMode_Bp.CurrentQuestionMode` (`self.OwningGameMode`))
        (:`NewEnumerator1`
          (if (`/Game/Main/BP/GameMode/GameplayGameMode_Bp.SelectedPlayerCanAnswerQuestion` _owninggamemode)
            _
            (else
              (`/Game/Main/BP/PlayerState/GamePlayPlayerState.RemoveStatus` (`/Game/Main/BP/PlayerController/GameplayPlayerController_BP.GetPlayer State` (`/Game/Main/BP/GameMode/GameplayGameMode_Bp.CurrentAnsweringPlayer` _owninggamemode)) "NewEnumerator3")
              (return "NewEnumerator18"))))
        (:`NewEnumerator0`
          _)
        (:`NewEnumerator2`
          _)
        (:`NewEnumerator4`
          _))
      (`/Game/Main/BP/GameMode/GameplayGameMode_Bp.ProcessAndSetQuestion` (`self.OwningGameMode`))
      (return "NewEnumerator5"))
    (:`NewEnumerator5`
      (return "NewEnumerator6"))
    (:`NewEnumerator6`
      (set `/Game/Main/BP/GameMode/GameplayGameMode_Bp.AcceptInput` false (`self.OwningGameMode`))
      (return "NewEnumerator7"))
    (:`NewEnumerator7`
      ;[1 1 1] Was it able to succesfully score the player, based on the mode move to the next phase,(normal will show landing spot if successful, others show mode winner), if failed, normal moves to resulting phase after checking round
      (if (`/Game/Main/BP/GameMode/GameplayGameMode_Bp.MarkSuccessful` (`self.OwningGameMode`))
        (switch `/Game/Main/Enums/Question/QuestionMode_Enum` (`/Game/Main/BP/GameMode/GameplayGameMode_Bp.CurrentQuestionMode` (`self.OwningGameMode`))
          (:`NewEnumerator1`
            (return "NewEnumerator21"))
          (:`NewEnumerator0`
            _)
          (:`NewEnumerator2`
            _)
          (:`NewEnumerator4`
            _))
        (return "NewEnumerator11")
        (else
          (switch `/Game/Main/Enums/Question/QuestionMode_Enum` (`/Game/Main/BP/GameMode/GameplayGameMode_Bp.CurrentQuestionMode` (`self.OwningGameMode`))
            (:`NewEnumerator1`
              (return "NewEnumerator21"))
            (:`NewEnumerator0`
              _)
            (:`NewEnumerator2`
              _)
            (:`NewEnumerator4`
              _))
          (return "NewEnumerator11"))))
    (:`NewEnumerator18`
      (bind _resultingphase (`/Game/Main/BP/GameMode/GameplayGameMode_Bp.Check Round Question and Next Answering Player` (`self.OwningGameMode`)))
      (return _resultingphase))
    (:`NewEnumerator8`
      ;[1 1 1] move to the next phase based on the current landing spot value
      (switch `/Game/Main/Enums/SpotEffect_Enum` (`/Game/Main/BP/GameMode/GameplayGameMode_Bp.CurrentQuestionPlayerLandingSpotEffect` (`self.OwningGameMode`))
        (:`NewEnumerator0`
          (`/Game/Main/BP/GameMode/GameplayGameMode_Bp.SetNextQuestionMode` (`self.OwningGameMode`) "NewEnumerator0")
          (return "NewEnumerator4"))
        (:`NewEnumerator1`
          (return "NewEnumerator9"))
        (:`NewEnumerator2`
          _)
        (:`NewEnumerator4`
          _)
        (:`NewEnumerator5`
          _)
        (:`NewEnumerator6`
          _))
      (bind _resultingphase_2 (`/Game/Main/BP/GameMode/GameplayGameMode_Bp.Check Round Question and Next Answering Player` (`self.OwningGameMode`)))
      (return _resultingphase_2))
    (:`NewEnumerator9`
      ;[1 1 1] Check the duel choice player made, if player wants to duel check if there is any player available for duel else, move to no duel phase
      (set `/Game/Main/BP/GameMode/GameplayGameMode_Bp.AcceptInput` false (`self.OwningGameMode`))
      (bind _willduel (`/Game/Main/BP/GameMode/GameplayGameMode_Bp.Check Duel Choice` (`self.OwningGameMode`)))
      (if _willduel
        (`/Game/Main/BP/GameMode/GameplayGameMode_Bp.AcceptDuel` (`self.OwningGameMode`))
        (if (`/Game/Main/BP/GameMode/GameplayGameMode_Bp.CheckForAvailableDuelablePlayers` (`self.OwningGameMode`))
          (return "NewEnumerator20")
          (else
            _))
        (else
          (`/Game/Main/BP/GameMode/GameplayGameMode_Bp.DuelCanceled` (`self.OwningGameMode`))))
      (return "NewEnumerator16"))
    (:`NewEnumerator10`
      (set `/Game/Main/BP/GameMode/GameplayGameMode_Bp.AcceptInput` false (`self.OwningGameMode`))
      (`/Game/Main/BP/GameMode/GameplayGameMode_Bp.CheckSelectedDueledPlayer` (`self.OwningGameMode`))
      (return "NewEnumerator17"))
    (:`NewEnumerator20`
      (return "NewEnumerator10"))
    (:`NewEnumerator16`
      (bind _resultingphase_3 (`/Game/Main/BP/GameMode/GameplayGameMode_Bp.Check Round Question and Next Answering Player` (`self.OwningGameMode`)))
      (return _resultingphase_3))
    (:`NewEnumerator17`
      (return "NewEnumerator4"))
    (:`NewEnumerator11`
      ;[1 1 1] Does question mode have a winner, select next phase based on this
      (switch `/Game/Main/Enums/Question/QuestionMode_Enum` (`/Game/Main/BP/GameMode/GameplayGameMode_Bp.CurrentQuestionMode` (`self.OwningGameMode`))
        (:`NewEnumerator0`
          (if _marksuccessful
            (return "NewEnumerator21")
            (else
              (`/Game/Main/BP/GameMode/GameplayGameMode_Bp.SetNextQuestionMode` (`self.OwningGameMode`) "NewEnumerator1")
              (bind _resultingphase_4 (`/Game/Main/BP/GameMode/GameplayGameMode_Bp.Check Round Question and Next Answering Player` (`self.OwningGameMode`)))
              (return _resultingphase_4))))
        (:`NewEnumerator2`
          (if _marksuccessful
            (return "NewEnumerator21")
            (else
              (return "NewEnumerator4"))))
        (:`NewEnumerator4`
          (if _marksuccessful
            (return "NewEnumerator21")
            (else
              (return "NewEnumerator4"))))))
    (:`NewEnumerator12`
      (return "NewEnumerator4"))
    (:`NewEnumerator13`
      (bind _resultphase (`/Game/Main/BP/GameMode/GameplayGameMode_Bp.GameOverNextPhase` (`self.OwningGameMode`)))
      (return _resultphase))
    (:`NewEnumerator21`
      (switch `/Game/Main/Enums/Question/QuestionMode_Enum` (`/Game/Main/BP/GameMode/GameplayGameMode_Bp.CurrentQuestionMode` (`self.OwningGameMode`))
        (:`NewEnumerator1`
          (if (`/Game/Main/BP/GameMode/GameplayGameMode_Bp.MarkSuccessful` (`self.OwningGameMode`))
            (return "NewEnumerator8")
            (else
              _)))
        (:`NewEnumerator0`
          _)
        (:`NewEnumerator2`
          _)
        (:`NewEnumerator4`
          (return "NewEnumerator14")))
      (`/Game/Main/BP/GameMode/GameplayGameMode_Bp.SetNextQuestionMode` (`self.OwningGameMode`) "NewEnumerator1")
      (bind _resultingphase_5 (`/Game/Main/BP/GameMode/GameplayGameMode_Bp.Check Round Question and Next Answering Player` (`self.OwningGameMode`)))
      (return _resultingphase_5))))