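; Game state for a multiplayer quiz game with rounds, category votes, duels and landing spots, holding the shared match data.
; Setters store that data and translate game phases into screen phases.
; RepNotifies push timers and screen changes to the local controller's UI, with the host getting a remapped screen and participants the raw phase.
; Helpers gather player states excluding the host and filter eligible duel opponents.
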(fn `ChangeLocalPlayerScreen`
  (bind _returnvalue (`GameplayStatics.GetPlayerController` 0))
  (if (and (`Controller.IsLocalPlayerController` _returnvalue) (`self.HasAuthority` _returnvalue))
    (bind _result (`self.Get Screen For Server`))
    (message `/Game/Main/BP/Interfaces/SCPlayerControllerInterface.UIShowScreen` _returnvalue _result)
    (else
      (bind _result_2 (`self.Get Screen For Participants`))
      (message `/Game/Main/BP/Interfaces/SCPlayerControllerInterface.UIShowScreen` _returnvalue _result_2))))

(fn `CurrentQuestionMode`
  (params (QuestionMode :type "/Game/Main/Enums/Question/QuestionMode_Enum Enum" :default "NewEnumerator1"))
  (set `self.QuestionMode` QuestionMode))

(fn `Get Screen For Participants`
  (returns (result :type "/Game/Main/Enums/ScreenPageType_Enum Enum"))
  (locals (ParticipantScreen :type "/Game/Main/Enums/ScreenPageType_Enum Enum" :default "NewEnumerator32"))
  (`|ExecutionSequence`
    (:`then_0`
      (set `local.ParticipantScreen` (`self.Screen Phase`)))
    (:`then_1`
      (return (`local.ParticipantScreen`)))))

(fn `Get Screen For Server`
  (returns (result :type "/Game/Main/Enums/ScreenPageType_Enum Enum"))
  (locals (ServerScreen :type "/Game/Main/Enums/ScreenPageType_Enum Enum" :default "NewEnumerator32"))
  (`|ExecutionSequence`
    (:`then_0`
      (bind _output_get (set `local.ServerScreen` (`self.Screen Phase`)))
      (switch `/Game/Main/Enums/ScreenPageType_Enum` _output_get
        (:`NewEnumerator2`
          (set `local.ServerScreen` "NewEnumerator32" :!label _label))
        (:`NewEnumerator10`
          (goto _label))
        (:`NewEnumerator17`
          (set `local.ServerScreen` "NewEnumerator7"))))
    (:`then_1`
      (return (`local.ServerScreen`)))))

(fn `GetDuelablePlayersInfo`
  (params (duelingplayer :type "/Game/Main/BP/PlayerState/GamePlayPlayerState Object Reference"))
  (returns (DuelablePlayersInfo :type "Array of /Game/Main/BP/PlayerState/GamePlayPlayerState Object Reference"))
  (locals (TempInformation :type "Array of /Game/Main/BP/PlayerState/GamePlayPlayerState Object Reference"))
  (for _array_element (`self.GetPlayerStatesCast`)
    (if (!= _array_element (`local.duelingplayer`))
      (if (and (not (`/Game/Main/BP/PlayerState/GamePlayPlayerState.FindStatusInPlayer` _array_element "NewEnumerator0")) (not (`/Game/Main/BP/PlayerState/GamePlayPlayerState.IsPlayerEliminated` _array_element)))
        (`KismetArrayLibrary.Array_AddUnique` (`local.TempInformation`) _array_element))))
  (return (`local.TempInformation`)))

(fn `GetPlayerStatesCast`
  (returns (Result :type "Array of /Game/Main/BP/PlayerState/GamePlayPlayerState Object Reference"))
  (locals (AllPlayerStates :type "Array of /Game/Main/BP/PlayerState/GamePlayPlayerState Object Reference") (TempRes :type "/Game/Main/BP/PlayerState/GamePlayPlayerState Object Reference"))
  (for _array_element (`self.PlayerArray`)
    (bind _asgame_play_player_state (cast `/Game/Main/BP/PlayerState/GamePlayPlayerState` _array_element))
    (bind _output_get (set `local.TempRes` _asgame_play_player_state))
    (bind _returnvalue (`PlayerState.GetPlayerController` _output_get))
    (if (not (and (`Controller.IsLocalPlayerController` _returnvalue) (`self.HasAuthority` _returnvalue)))
      (`KismetArrayLibrary.Array_Add` (`local.AllPlayerStates`) (`local.TempRes`))))
  (return (`local.AllPlayerStates`)))

(fn `GetQuestionTime`
  (returns (Time :type Integer))
  (return 0))

(fn `OnRep_CategoryTimer`
  (`self.UpdateCategoryTimeForPlayers`))

(fn `OnRep_QuestionTime`
  (`self.UpdateTimeForPlayer`))

(fn `OnRep_Screen Phase`
  (`self.ChangeLocalPlayerScreen`))

(fn `OnRep_TimeLeftToShowOptions`
  (message `/Game/Main/BP/Interfaces/SCPlayerControllerInterface.UpdateUITimer` (`GameplayStatics.GetPlayerController` 0) (`self.TimeLeftToShowOptions`)))

(fn `OnRep_TimeLeftToShowQuestionScreen`)

(fn `Set Current Category`
  (params (SelectedCategory :type "/Game/Main/Enums/Question/QuestionsCategory_Enum Enum" :default "NewEnumerator0"))
  (set `self.SelectedCategory` SelectedCategory))

(fn `Set Current Landing Spot`
  (params (Spot :type "/Game/Main/Enums/SpotEffect_Enum Enum" :default "NewEnumerator0"))
  (set `self.CurrentLandingSpot` Spot))

(fn `Set Current Question`
  (params (Question :type "/Game/Main/Structs/QuestionStructs/QuestionStruct Structure"))
  (set `self.Question` Question))

(fn `Set Current Round No`
  (params (`Round No` :type Integer))
  (set `self.Round No` `Round No`))

(fn `Set Phase Time`
  (params (PhaseTime :type "Float (double-precision)"))
  (set `self.PhaseTime` PhaseTime))

(fn `Set Screen Phase`
  (params (GamePhase :type "/Game/Main/Enums/GamePhase_Enum Enum" :default "NewEnumerator0"))
  (switch `/Game/Main/Enums/GamePhase_Enum` (`local.GamePhase`)
    (:`NewEnumerator0`
      (set `self.Screen Phase` "NewEnumerator19"))
    (:`NewEnumerator1`
      (set `self.Screen Phase` "NewEnumerator0"))
    (:`NewEnumerator2`
      (set `self.Screen Phase` "NewEnumerator3"))
    (:`NewEnumerator3`
      (set `self.Screen Phase` "NewEnumerator5"))
    (:`NewEnumerator19`
      (set `self.Screen Phase` "NewEnumerator33"))
    (:`NewEnumerator4`
      (set `self.Screen Phase` "NewEnumerator16"))
    (:`NewEnumerator5`
      (set `self.Screen Phase` "NewEnumerator17"))
    (:`NewEnumerator6`
      (set `self.Screen Phase` "NewEnumerator7"))
    (:`NewEnumerator7`
      (set `self.Screen Phase` "NewEnumerator8"))
    (:`NewEnumerator18`
      (set `self.Screen Phase` "NewEnumerator34"))
    (:`NewEnumerator8`
      (set `self.Screen Phase` "NewEnumerator1"))
    (:`NewEnumerator20`
      (set `self.Screen Phase` "NewEnumerator6"))
    (:`NewEnumerator16`
      (set `self.Screen Phase` "NewEnumerator31"))
    (:`NewEnumerator17`
      (set `self.Screen Phase` "NewEnumerator11"))
    (:`NewEnumerator11`
      (set `self.Screen Phase` "NewEnumerator12"))
    (:`NewEnumerator12`
      (set `self.Screen Phase` "NewEnumerator13"))
    (:`NewEnumerator13`
      (set `self.Screen Phase` "NewEnumerator15"))
    (:`NewEnumerator14`
      (set `self.Screen Phase` "NewEnumerator14"))
    (:`NewEnumerator21`
      (set `self.Screen Phase` "NewEnumerator41"))))

(fn `Set Selectable Categories `
  (params (Categories :type "Array of /Game/Main/Enums/Question/QuestionsCategory_Enum Enum"))
  (set `self.Categories` Categories))

(fn `SetCurrentQuestionNo`
  (params (QuestionNo :type Integer))
  (set `self.QuestionNo` QuestionNo))

(fn `SetDuelablePlayersState`
  (params (DuelablePlayers :type "Array of /Game/Main/BP/PlayerState/GamePlayPlayerState Object Reference"))
  (set `self.DuelablePlayersState` DuelablePlayers))

(fn `SetDuelChoiceAndDuelInfo`
  (params (DuelChoiceAndDuelInfo :type "/Game/Main/Structs/BoolToPlayerInfo_Struct Structure"))
  (set `self.DuelChoiceAndDuelInfo` DuelChoiceAndDuelInfo))

(fn `SetLandingSpots`
  (params (LandingSpots :type "Array of /Game/Main/Enums/SpotEffect_Enum Enum"))
  (set `self.AvailableLandingSpots` LandingSpots))

(fn `SetLbInfo`
  (params (LBInfo :type "Array of /Game/Main/Structs/PlayerToStoredInt_Struct Structure"))
  (set `self.CurrentLBInfo` LBInfo))

(fn `SetModeInfoPlayerStates`
  (params (PlayersInMode :type "Array of /Game/Main/BP/PlayerController/GameplayPlayerController_BP Object Reference"))
  (locals (TempArray :type "Array of /Game/Main/BP/PlayerState/GamePlayPlayerState Object Reference"))
  (if (`KismetArrayLibrary.Array_IsNotEmpty` PlayersInMode)
    (for _array_element PlayersInMode
      (bind _asscplayer_state (`/Game/Main/BP/PlayerController/GameplayPlayerController_BP.GetPlayer State` _array_element))
      (`/Engine/EditorBlueprintResources/StandardMacros.IsValid` _asscplayer_state
        (:`Is Valid`
          (`KismetArrayLibrary.Array_Add` (`local.TempArray`) _asscplayer_state))))
    (set `self.ModePlayersState` (`local.TempArray`))))

(fn `SetModeWinner`
  (params (ModeWinnerAndInfo :type "/Game/Main/Structs/BoolToPlayerInfo_Struct Structure"))
  (set `self.ModeWinnerAndInfo` ModeWinnerAndInfo))

(fn `UpdateCategoryTimeForPlayers`
  (message `/Game/Main/BP/Interfaces/SCPlayerControllerInterface.UpdateUITimer` (`GameplayStatics.GetPlayerController` 0) (`self.CategoryTimer`)))

(fn `UpdateTimeForPlayer`
  (message `/Game/Main/BP/Interfaces/SCPlayerControllerInterface.UpdateUITimer` (`GameplayStatics.GetPlayerController` 0) (`self.QuestionTime`)))

(fn `UserConstructionScript`)