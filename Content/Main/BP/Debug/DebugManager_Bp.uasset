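; Debug manager owned by the host's player controller that lets a debug panel manipulate a multiplayer quiz game.
; Setup creates the debug widget, adds it through the UI manager and binds new-player joins to refresh its player selection buttons.
; Its events forward commands to the gameplay game mode, UI manager and players to control screens, question modes, rounds and phases, categories, answering player, landing spots, statuses and leaderboard.
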(event `SetupDebugManager`
  (bind _returnvalue (`GameplayStatics.GetGameMode`))
  (bind _asbase_player_controller_bp (cast `/Game/Main/BP/PlayerController/BasePlayerController_Bp` (`self.GetOwner`)))
  (set `self.HostController` _asbase_player_controller_bp)
  (bind _returnvalue_2 (`|CreateWidget` (`self.DebugClassUi`) (`self.HostController`) self (`/Game/Main/BP/PlayerController/BasePlayerController_Bp.UIManager` (`self.HostController`))))
  (set `self.DebugUiRef` _returnvalue_2)
  (`/Game/Main/BP/Components/UIManager.AddDebugPanel` (`/Game/Main/BP/PlayerController/BasePlayerController_Bp.UIManager` (`self.HostController`)) (`self.DebugUiRef`))
  (`/Engine/EditorBlueprintResources/StandardMacros.IsValid` _returnvalue
    (:`Is Valid`
      (bind _asgameplay_game_mode_bp (cast `/Game/Main/BP/GameMode/GameplayGameMode_Bp` _returnvalue))
      (set `self.GameMode` _asgameplay_game_mode_bp)
      (add `/Game/Main/BP/GameMode/GameplayGameMode_Bp.ForDebugNewPlayerJoin` (`self.GameMode`) (delegate `RefreshEditablePlayers`)))))

(event `RefreshEditablePlayers`
  (`/Game/Main/UI/DebugScreen/DebugUi_Host.UpdatePlayersSelectionButton` (`self.DebugUiRef`) (`/Game/Main/BP/GameMode/GameplayGameMode_Bp.NonEliminatedPlayers` (`self.GameMode`))))

(event `ChangeScreenForHost`
  (params (Screen :type "/Game/Main/Enums/ScreenPageType_Enum Enum" :default "NewEnumerator0"))
  (`/Game/Main/BP/Components/UIManager.Show Page Screen` (`/Game/Main/BP/PlayerController/BasePlayerController_Bp.UIManager` (`self.HostController`)) Screen))

(event `ChangePlayerType`
  (params (NewPlayerType :type "/Game/Main/Enums/PlayerType Enum" :default "NewEnumerator2"))
  (`/Game/Main/BP/Components/UIManager.Debug_ChangePlayerType_Screen` (`/Game/Main/BP/PlayerController/BasePlayerController_Bp.UIManager` (`self.HostController`)) NewPlayerType))

(event `Debug_CheckRound`
  (`/Game/Main/BP/GameMode/GameplayGameMode_Bp.Debug_CheckNextPlayerAndRound` (`self.GameMode`)))

(event `Debug_ChangeQuestionMode`
  (params (Mode :type "/Game/Main/Enums/Question/QuestionMode_Enum Enum" :default "NewEnumerator1"))
  (bind _gamemode (`self.GameMode`))
  (switch `/Game/Main/Enums/Question/QuestionMode_Enum` Mode
    (:`NewEnumerator1`
      (`/Game/Main/BP/GameMode/GameplayGameMode_Bp.Debug_NormalQuestion` _gamemode))
    (:`NewEnumerator0`
      (`/Game/Main/BP/GameMode/GameplayGameMode_Bp.Debug_BonusStart` _gamemode))
    (:`NewEnumerator2`
      (`/Game/Main/BP/GameMode/GameplayGameMode_Bp.Debug_DuelStart` _gamemode))
    (:`NewEnumerator4`
      (`/Game/Main/BP/GameMode/GameplayGameMode_Bp.Debug_TryTiebreaker` _gamemode))))

(event `Debug_RefreshLb`
  (`/Game/Main/BP/GameMode/GameplayGameMode_Bp.CalculateAndSetLeaderboard` (`self.GameMode`)))

(event `Debug_ShowAvailableSpotsForCurrentPlayer`
  (params (PlayerToProcessFor :type "/Game/Main/BP/PlayerController/GameplayPlayerController_BP Object Reference"))
  (`/Game/Main/BP/GameMode/GameplayGameMode_Bp.ProcessAvailableLandingSpots` (`self.GameMode`) PlayerToProcessFor))

(event `Debug_IncrementRound`
  (bind _gamemode (`self.GameMode`))
  (if (>= (`/Game/Main/BP/GameMode/GameplayGameMode_Bp.CurrentRoundNo` _gamemode) (`/Game/Main/BP/GameMode/GameplayGameMode_Bp.MaxRoundCount` _gamemode))
    (set `/Game/Main/BP/GameMode/GameplayGameMode_Bp.CurrentRoundNo` 0 _gamemode))
  (`/Game/Main/BP/GameMode/GameplayGameMode_Bp.Debug_ChangePhase` (`self.GameMode`) "NewEnumerator1"))

(event `SetAnsweringPlayer`
  (params (SelectedPlayer :type "/Game/Main/BP/PlayerController/GameplayPlayerController_BP Object Reference"))
  (set `/Game/Main/BP/GameMode/GameplayGameMode_Bp.CurrentAnsweringPlayer` SelectedPlayer (`self.GameMode`)))

(event `Debug _ ShowQuestionForNextAnsweringPlayer`
  (`/Game/Main/BP/GameMode/GameplayGameMode_Bp.Debug_CheckNextPlayerAndRound` (`self.GameMode`)))

(event `Debug_SetCateogry`
  (params (Category :type "/Game/Main/Enums/Question/QuestionsCategory_Enum Enum" :default "NewEnumerator0"))
  (set `/Game/Main/BP/GameMode/GameplayGameMode_Bp.CurrentCategory` Category (`self.GameMode`)))

(event `Debug_AddStatusToPlayer`
  (params (PlayerToAdd :type "/Game/Main/BP/PlayerController/GameplayPlayerController_BP Object Reference") (StatusToAdd :type "/Game/Main/Enums/Status_Enum Enum" :default "NewEnumerator0"))
  (`/Engine/EditorBlueprintResources/StandardMacros.IsValid` PlayerToAdd
    (:`Is Valid`
      (`/Game/Main/BP/PlayerState/GamePlayPlayerState.AddStatusToPlayer` (`/Game/Main/BP/PlayerController/GameplayPlayerController_BP.GetPlayer State` PlayerToAdd) StatusToAdd))))

(event `ChangeScreenForPlayer`
  (params (SelectedPlayer :type "/Game/Main/BP/PlayerController/GameplayPlayerController_BP Object Reference") (Screen :type "/Game/Main/Enums/ScreenPageType_Enum Enum" :default "NewEnumerator0"))
  (`/Engine/EditorBlueprintResources/StandardMacros.IsValid` SelectedPlayer
    (:`Is Valid`
      (`/Game/Main/BP/PlayerController/GameplayPlayerController_BP.ShowScreen` SelectedPlayer Screen))))

(event `Collate categories`
  (`/Game/Main/BP/GameMode/GameplayGameMode_Bp.Debug_ChangePhase` (`self.GameMode`) "NewEnumerator3"))

(event `Debug_RemoveStatusFromPlayer`
  (params (Target :type "/Game/Main/BP/PlayerController/GameplayPlayerController_BP Object Reference") (StatusToRemove :type "/Game/Main/Enums/Status_Enum Enum" :default "NewEnumerator0"))
  (`/Engine/EditorBlueprintResources/StandardMacros.IsValid` Target
    (:`Is Valid`
      (`/Game/Main/BP/PlayerState/GamePlayPlayerState.RemoveStatus` (`/Game/Main/BP/PlayerController/GameplayPlayerController_BP.GetPlayer State` Target) StatusToRemove))))

(event `ChangeScreenForAllPlayers`
  (params (ScreenType :type "/Game/Main/Enums/ScreenPageType_Enum Enum" :default "NewEnumerator0"))
  (for _array_element (`/Game/Main/BP/GameMode/GameplayGameMode_Bp.AllConnectedPlayers` (`self.GameMode`))
    (`/Game/Main/BP/PlayerController/GameplayPlayerController_BP.ShowScreen` _array_element ScreenType)))

(event `Debug_MarkQuestion`
  (`/Game/Main/BP/GameMode/GameplayGameMode_Bp.DebugMode_MarkQuestion` (`self.GameMode`)))

(event `Debug_ShowSpotForPlayer`
  (params (Spot :type "/Game/Main/Enums/SpotEffect_Enum Enum" :default "NewEnumerator0"))
  (bind _gamemode (`self.GameMode`))
  (set `/Game/Main/BP/GameMode/GameplayGameMode_Bp.CurrentQuestionPlayerLandingSpotEffect` Spot _gamemode)
  (`/Game/Main/BP/GameMode/GameplayGameMode_Bp.Debug_ShowSpot` _gamemode))