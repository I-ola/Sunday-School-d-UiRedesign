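; Player controller for a multiplayer quiz game with category votes, duels, player statuses and a spectator view.
; On local BeginPlay it creates the gameplay screen through UIManager and copies the game instance's profile into the player state.
; UI choices and answers go through InformServer events to game mode messages, while incoming events update screens, leaderboard, votes and landing spots.
; It can also create a LAN session and open the Gameplay level as listen server.
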(event `CreateGame`
  (`CreateSessionCallbackProxy.CreateSession` self 2 true
    (:`OnSuccess`
      (`GameplayStatics.OpenLevel` "Gameplay" false "?listen"))))

(event `SetupPlayer`
  (params (IsSpectator :type Boolean))
  ;[1 1 1] 1. called from game mode
)

(event `self.ReceiveBeginPlay`
  ;[1 1 1] 1
  (if (`self.IsLocalPlayerController`)
    (set `/Game/Main/BP/Components/UIManager.OwningPlayerController` self (`self.UIManager`))
    (set `self.bShowMouseCursor` true)
    (`/Game/Main/BP/Components/UIManager.CreateMainScreen_Gameplay` (`self.UIManager`))
    (bind _asscgame_instance (cast `/Game/Main/SCGameInstance` (`GameplayStatics.GetGameInstance`)))
    (`self.SetupRef` (`/Game/Main/SCGameInstance.Get Player Profile Info` _asscgame_instance))))

(event `SetupRef`
  (params (PlayerProfile :type "/Game/Main/Structs/ProfileInfo_Struct Structure"))
  ;[1 1 1] 2
  (`/Game/Main/BP/PlayerState/GamePlayPlayerState.SetPlayerInfo` (`self.GetPlayer State`) PlayerProfile)
  (bind _asgameplay_game_mode_bp (cast `/Game/Main/BP/GameMode/GameplayGameMode_Bp` (`GameplayStatics.GetGameMode`)))
  (`/Game/Main/BP/GameMode/GameplayGameMode_Bp.ForDebugNewPlayerJoin` _asgameplay_game_mode_bp))

(event `/Game/Main/BP/Interfaces/SCPlayerControllerInterface.StartButtonClicked`
  (bind _returnvalue (`GameplayStatics.GetGameMode`))
  ;[1 1 1] called from spectator view lobby screen
  (`/Engine/EditorBlueprintResources/StandardMacros.IsValid` _returnvalue
    (:`Is Valid`
      (message `/Game/Main/BP/Interfaces/SCGameModeInterface.StartGame` _returnvalue))
    (:`Is Not Valid`
      (`KismetSystemLibrary.PrintString` "Not found mode"))))

(event `UpdateStreaksUI`
  (params (StreakCount :type Integer))
  ;[1 1 1] Update the UI that shows the amount of questions player has gotten correct consecutively
)

(event `/Game/Main/BP/Interfaces/SCPlayerControllerInterface.Ui on Select Duel Partner`
  (params (SelectedPlayer :type "/Game/Main/BP/PlayerState/GamePlayPlayerState Object Reference"))
  ;[1 1 1] Called from the duel ui
  (`self.InformServerOfSelectedDuelPartner` SelectedPlayer))

(event `/Game/Main/BP/Interfaces/SCPlayerControllerInterface.OnDuelOptionSelected`
  (params (ChoseToDuel :type Boolean) (SelectedCategory :type "/Game/Main/Enums/Question/QuestionsCategory_Enum Enum" :default "NewEnumerator0"))
  ;[1 1 1] Called from the duel ui
  ;;[1 1 1] called from player ui duel choice ui
  (`self.InformServerOfPlayerDuel` ChoseToDuel SelectedCategory))

(event `InformServerOfPlayerDuel`
  (params (ChoseToDuel :type Boolean) (SelectedCategory :type "/Game/Main/Enums/Question/QuestionsCategory_Enum Enum" :default "NewEnumerator0"))
  ;[1 1 1] Called from the duel ui
  (message `/Game/Main/BP/Interfaces/SCGameModeInterface.ChoseToDuel` (`GameplayStatics.GetGameMode`) ChoseToDuel SelectedCategory))

(event `/Game/Main/BP/Interfaces/SCPlayerControllerInterface.QuestionAnswered`
  (params (CorrectAnswer :type Boolean) (Time :type Integer) (SelectedOption :type "/Game/Main/Enums/OptionsButtons_Enum Enum" :default "NewEnumerator0"))
  ;[1 1 1] called from the question ui after an option has been clicked
  (`self.InformServerPlayerAnsweredQuestion` Time CorrectAnswer SelectedOption))

(event `InformServerPlayerAnsweredQuestion`
  (params (Time :type Integer) (IsCorrect :type Boolean) (SelectedOption :type "/Game/Main/Enums/OptionsButtons_Enum Enum" :default "NewEnumerator0"))
  ;[1 1 1] called from the question ui after an option has been clicked
  (message `/Game/Main/BP/Interfaces/SCGameModeInterface.QuestionAnswered` (`GameplayStatics.GetGameMode`) self Time IsCorrect SelectedOption))

(event `InformServerOfSelectedDuelPartner`
  (params (SelectedDuelPartner :type "/Game/Main/BP/PlayerState/GamePlayPlayerState Object Reference"))
  ;[1 1 1] Called from the duel ui
  (message `/Game/Main/BP/Interfaces/SCGameModeInterface.DuelPartnerSelected` (`GameplayStatics.GetGameMode`) SelectedDuelPartner))

(event `UpdateLB(Spec)`
  (params (LbInfo :type "Array of /Game/Main/Structs/PlayerToStoredInt_Struct Structure"))
  ;[1 1 1] Update lb on spectator view only
  (`/Game/Main/UI/Base/MainScreens/BaseScreen.UpdateLbUi` (`/Game/Main/BP/Components/UIManager.MainScreen` (`self.UIManager`)) LbInfo))

(event `ShowAvailableLandingSpot(Spec)`
  (params (AvailableSpots :type "Array of /Game/Main/Enums/SpotEffect_Enum Enum"))
  ;[1 1 1] Show the spots player can land on spec screen
  (`/Game/Main/UI/Base/MainScreens/BaseScreen.SetupLandingSpots` (`/Game/Main/BP/Components/UIManager.MainScreen` (`self.UIManager`)) AvailableSpots))

(event `/Game/Main/BP/Interfaces/SCPlayerControllerInterface.OnRoundCategorySelectionButtonClicked`
  (params (SelectedCategory :type "/Game/Main/Enums/Question/QuestionsCategory_Enum Enum" :default "NewEnumerator0"))
  ;[1 1 1] called from round category selection ui
  (`self.InformServerOfSelectedCategoryForRound` SelectedCategory))

(event `OnStatusAdded`
  (params (AddedStatus :type "/Game/Main/Enums/Status_Enum Enum" :default "NewEnumerator0"))
  (`/Game/Main/BP/Components/UIManager.Show Page Screen` (`self.UIManager`) (select `/Game/Main/Enums/Status_Enum` AddedStatus :`NewEnumerator0` "NewEnumerator27" :`NewEnumerator1` "NewEnumerator21" :`NewEnumerator2` "NewEnumerator22" :`NewEnumerator3` "NewEnumerator29" :`NewEnumerator4` "NewEnumerator20" :!type "/Game/Main/Enums/ScreenPageType_Enum Enum")))

(event `OnStatusRemoved`
  (params (RemovedStatus :type "/Game/Main/Enums/Status_Enum Enum" :default "NewEnumerator0"))
  (`/Game/Main/BP/Components/UIManager.Show Page Screen` (`self.UIManager`) (select `/Game/Main/Enums/Status_Enum` RemovedStatus :`NewEnumerator0` "NewEnumerator28" :`NewEnumerator1` "NewEnumerator25" :`NewEnumerator2` "NewEnumerator26" :`NewEnumerator3` "NewEnumerator30" :`NewEnumerator4` "NewEnumerator24" :!type "/Game/Main/Enums/ScreenPageType_Enum Enum")))

(event `InformServerOfSelectedCategoryForRound`
  (params (SelectedCategory :type "/Game/Main/Enums/Question/QuestionsCategory_Enum Enum" :default "NewEnumerator0"))
  ;[1 1 1] called from round category selection ui
  (message `/Game/Main/BP/Interfaces/SCGameModeInterface.OnSelectCategory` (`GameplayStatics.GetGameMode`) SelectedCategory self))

(event `AddPlayerCategoryVotes`
  (params (CategoryAndVote :type "/Game/Main/Enums/Question/QuestionsCategory_Enum Enum" :default "NewEnumerator0") (SelectingPlayer :type "/Game/Main/Structs/ProfileInfo_Struct Structure"))
  ;[1 1 1] Add the votes to the respective category (spectator view only)
  (`/Game/Main/UI/Base/MainScreens/BaseScreen.UpdateVotesScreen` (`/Game/Main/BP/Components/UIManager.MainScreen` (`self.UIManager`)) CategoryAndVote SelectingPlayer))

(event `UpdateAnswerSelectionProfile(Spec)`
  (params (SelectedOption :type "/Game/Main/Enums/OptionsButtons_Enum Enum" :default "NewEnumerator0") (Player :type "/Game/Main/Structs/ProfileInfo_Struct Structure"))
  ;[1 1 1] Update the profiles on the answer options to show what player selects (only spectator view)
  (`/Game/Main/UI/Base/MainScreens/BaseScreen.UpdatePlayerSelectedAnswer` (`/Game/Main/BP/Components/UIManager.MainScreen` (`self.UIManager`)) SelectedOption Player))

(event `ShowScreen`
  (params (ScreenToShow :type "/Game/Main/Enums/ScreenPageType_Enum Enum" :default "NewEnumerator0"))
  ;[1 1 1] Show any screen passed here, for gameover setup the screen for spec mode and none spec mode (round category vote info should do this too)
  (`/Game/Main/BP/Components/UIManager.Show Page Screen` (`self.UIManager`) ScreenToShow))

(event `/Game/Main/BP/Interfaces/SCPlayerControllerInterface.UIShowScreen`
  (params (Screen :type "/Game/Main/Enums/ScreenPageType_Enum Enum" :default "NewEnumerator32"))
  ;[1 1 1] called from gamestate repnotify
  (`self.ShowScreen` Screen))

(event `RefreshLobbyScreen`
  ;[1 1 1] called when playerstate has stored the player info on sever side
  (bind _mainscreen (`/Game/Main/BP/Components/UIManager.MainScreen` (`self.UIManager`))
    (:`then`
      (`/Game/Main/UI/Base/MainScreens/BaseScreen.RefreshLobby` _mainscreen))
    (:`else`)))

(event `SetCategoryForUI`
  (params (categories :type "Array of /Game/Main/Enums/Question/QuestionsCategory_Enum Enum (by ref)"))
  (`/Game/Main/UI/Base/MainScreens/BaseScreen.SetCategoriesForCurrentScreen` (`/Game/Main/BP/Components/UIManager.MainScreen` (`self.UIManager`)) categories))

(fn `GetPlayer State`
  (returns (`AsSCPlayer State` :type "/Game/Main/BP/PlayerState/GamePlayPlayerState Object Reference"))
  (bind _asgame_play_player_state (cast `/Game/Main/BP/PlayerState/GamePlayPlayerState` (`self.PlayerState`))
    (:`then`
      (return _asgame_play_player_state))
    (:`CastFailed`
      (`KismetSystemLibrary.PrintString` "Helloooooooooo"))))

(fn `UserConstructionScript`)